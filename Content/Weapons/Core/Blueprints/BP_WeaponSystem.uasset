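; Weapon system Blueprint that handles player shooting, ammo and reloading through Enhanced Input.
; Shots are cone-spread line traces with debug drawing: Realistic mode traces from the muzzle and applies damage, while Arcade traces from the camera without damage.
; Each trace spends ammo and re-enters firing through AutomaticFire, delayed by fire rate, or SemiFire, immediately.
; Delayed reloads distinguish empty, open-bolt and tactical plus-one cases, without drawing on reserve ammo.
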(event `self.ReceiveTick`
  (params (DeltaSeconds :type "Float (single-precision)"))
  (`|ExecutionSequence`
    (:`then_0`
      (`self.Debug`))
    (:`then_1`
      (if (< (`self.CurrentAmmo`) 0)
        (set `self.CurrentAmmo` 0)))))

(event `self.ReceiveBeginPlay`
  (`self.Init`)
  (`self.Debug`))

(event `EnhancedInput|/Game/Core/Input/Actions/Weapon/IA_Shoot`
  (params (ActionValue :type Boolean) (ElapsedSeconds :type "Float (double-precision)") (TriggeredSeconds :type "Float (double-precision)") (InputAction :type "InputAction Object Reference" :default "/Game/Core/Input/Actions/Weapon/IA_Shoot.IA_Shoot"))
  (:`Started`
    (set `self.IsShooting` true)
    (if (> (`self.CurrentAmmo`) 0)
      (if (`self.CanFire`)
        (if (`self.IsRealistic`)
          (`self.RealisticFire`)
          (else
            (`self.ArcadeFire`))))
      (else
        (set `self.CanFire` false))))
  (:`Completed`
    (set `self.IsShooting` false)))

(event `EnhancedInput|/Game/Core/Input/Actions/Weapon/IA_Reload`
  (params (ActionValue :type Boolean) (ElapsedSeconds :type "Float (double-precision)") (TriggeredSeconds :type "Float (double-precision)") (InputAction :type "InputAction Object Reference" :default "/Game/Core/Input/Actions/Weapon/IA_Reload.IA_Reload"))
  ;[1 1 1] Reload
  (:`Triggered`
    (if (not (`self.IsReloading`))
      (set `self.IsReloading` true)
      (set `self.CanFire` false)
      (if (== (`self.CurrentAmmo`) 0)
        (set `self.CurrentAmmo` (`self.MaxAmmo`))
        (`KismetSystemLibrary.Delay` (`self.ReloadSpeed`) :!label _label)
        (set `self.IsReloading` false)
        (set `self.CanFire` true)
        (elif (`self.IsOpenBolt`)
          (set `self.CurrentAmmo` (`self.MaxAmmo`))
          (goto _label)
          (else
            (set `self.CurrentAmmo` (+ (`self.MaxAmmo`) 1))
            (`KismetSystemLibrary.Delay` (`self.TacticalReloadSpeed`))
            (set `self.IsReloading` false)
            (set `self.CanFire` true))))
      (`KismetSystemLibrary.PrintString` "Reload Complete"))))

(event `AutomaticFire`
  (if (`self.IsShooting`)
    (if (`self.CanFire`)
      (`KismetSystemLibrary.Delay` (`self.FireRate`))
      (if (`self.IsRealistic`)
        (`self.RealisticFire`)
        (else
          (`self.ArcadeFire`)))
      (else
        (set `self.IsShooting` false)))))

(event `SemiFire`
  (if (`self.IsRealistic`)
    (`self.RealisticFire`)
    (else
      (`self.ArcadeFire`))))

(fn `ArcadeFire`
  (bind _firstpersoncamera (`/Game/Core/BP_PlayerCharacter.FirstPersonCamera` (`self.PlayerReference`)))
  (bind _returnvalue (`SceneComponent.K2_GetComponentLocation` _firstpersoncamera))
  (if (> (`self.CurrentAmmo`) 0)
    (for _ (range 1 (+ (`self.BulletsPerClick`) 1))
      (`KismetSystemLibrary.LineTraceSingle` :`Start` _returnvalue :`End` (+ _returnvalue (* (`KismetMathLibrary.RandomUnitVectorInConeInDegrees` (`KismetMathLibrary.GetForwardVector` (`SceneComponent.K2_GetComponentRotation` _firstpersoncamera)) (`self.ArcadeSpread`)) (`self.ArcadeRange`))) :`TraceChannel` "TraceTypeQuery1" :`DrawDebugType` "ForDuration" :`DrawTime` 1.0)
      (set `self.BulletsPerClick` (`self.StoredBPC`))
      (`/Engine/EditorBlueprintResources/StandardMacros.DecrementInt` (`self.CurrentAmmo`)
        (:`  `
          (if (== (`KismetMathLibrary.Conv_ByteToInt` (`self.FireMode`)) 0)
            (`self.AutomaticFire`)
            (else
              (`self.SemiFire`))))))
    (else
      (set `self.CanFire` false))))

(fn `Debug`)

(fn `Init`
  (bind _returnvalue (`GameplayStatics.GetPlayerController` 0))
  (`self.EnableInput` _returnvalue)
  (`EnhancedInputSubsystemInterface.AddMappingContext` (pcsubsystem `EnhancedInputLocalPlayerSubsystem` _returnvalue) "/Game/Core/Input/IMC_Weapons.IMC_Weapons" 0 (struct))
  (set `self.CurrentAmmo` (`self.MaxAmmo`))
  (bind _asbp_player_character (cast `/Game/Core/BP_PlayerCharacter` (`GameplayStatics.GetPlayerCharacter` 0)))
  (set `self.PlayerReference` _asbp_player_character)
  (set `self.FireRate` (/ 60 (`self.RealFireRate`)))
  (set `self.CanFire` true)
  (set `self.StoredBPC` (`self.BulletsPerClick`))
  (set `self.ReserveAmmo` (* (`self.MaxAmmo`) 4)))

(fn `RealisticFire`
  (bind _muzzle (`/Game/Core/BP_PlayerCharacter.Muzzle` (`self.PlayerReference`)))
  (bind _returnvalue (`SceneComponent.K2_GetComponentLocation` _muzzle))
  (if (> (`self.CurrentAmmo`) 0)
    (for _ (range 1 (+ (`self.BulletsPerClick`) 1))
      (bind _outhit (`KismetSystemLibrary.LineTraceSingle` :`Start` _returnvalue :`End` (+ _returnvalue (* (`KismetMathLibrary.RandomUnitVectorInConeInDegrees` (`SceneComponent.GetForwardVector` _muzzle) (`self.RealisticSpread`)) (`self.RealisticRange`))) :`TraceChannel` "TraceTypeQuery1" :`DrawDebugType` "ForDuration" :`DrawTime` 1.0))
      (`|ExecutionSequence`
        (:`then_0`
          (set `self.BulletsPerClick` (`self.StoredBPC`))
          (`/Engine/EditorBlueprintResources/StandardMacros.DecrementInt` (`self.CurrentAmmo`)
            (:`  `
              (if (== (`KismetMathLibrary.Conv_ByteToInt` (`self.FireMode`)) 0)
                (`self.AutomaticFire`)
                (else
                  (`self.SemiFire`))))))
        (:`then_1`
          (`GameplayStatics.ApplyDamage` (`.HitActor` (`GameplayStatics.BreakHitResult` _outhit)) (`self.RealisticDamage`) null (`self.PlayerReference`)))))
    (else
      (set `self.CanFire` false))))

(fn `UserConstructionScript`)