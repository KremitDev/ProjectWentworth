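; Base enemy actor that tracks health, takes damage and is destroyed when health runs out.
; Init fills health to maximum and caches references to the player character and the BP_StatTrack actor.
; AnyDamage subtracts health, shows a hitmarker widget with sound for player-caused hits, then calls KillEnemy at zero or below.
; KillEnemy increments the stat tracker's kill counter when the player caused the damage, then destroys the actor.
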(event `self.ReceiveBeginPlay`
  (`self.Init`))

(event `self.ReceiveAnyDamage`
  (params (Damage :type "Float (single-precision)") (DamageType :type "DamageType Object Reference") (InstigatedBy :type "Controller Object Reference") (DamageCauser :type "Actor Object Reference"))
  (bind _output_get (set `self.CurrentHealth` (- (`self.CurrentHealth`) Damage)))
  (`|ExecutionSequence`
    (:`then_0`
      (if (== DamageCauser (`self.PlayerReference`))
        (`GameplayStatics.PlaySound2D` "/Game/Weapons/Sounds/A_Hitmarker_Cue.A_Hitmarker_Cue" 1.0 1.0 0.0 null null)
        (bind _returnvalue (`|CreateWidget` "/Game/Core/UserInterface/Gameplay/WB_Hitmarker.WB_Hitmarker_C"))
        (`UserWidget.AddToViewport` _returnvalue 0)))
    (:`then_1`
      (if (<= _output_get 0.0)
        (`self.KillEnemy`)))))

(event `KillEnemy`
  (if (== (stale `self.ReceiveAnyDamage` DamageCauser) (`self.PlayerReference`))
    (`/Engine/EditorBlueprintResources/StandardMacros.IncrementInt` (`/Game/Core/BP_StatTrack.KillCounter` (`self.StatsReference`))
      (:`  `
        _)))
  (`self.K2_DestroyActor`))

(fn `Init`
  (set `self.CurrentHealth` (`self.MaxHealth`))
  (set `self.bCanBeDamaged` true)
  (bind _asbp_player_character (cast `/Game/Core/Player/BP_PlayerCharacter` (`GameplayStatics.GetPlayerCharacter` 0)))
  (set `self.PlayerReference` _asbp_player_character)
  (bind _returnvalue (`GameplayStatics.GetActorOfClass` "/Game/Core/BP_StatTrack.BP_StatTrack_C"))
  (bind _asbp_stat_track (cast `/Game/Core/BP_StatTrack` _returnvalue))
  (set `self.StatsReference` _asbp_stat_track))

(fn `UserConstructionScript`)