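; Ammo pickup actor that adds ammo to the player's weapon when the player touches it.
; On BeginPlay it casts player 0's character to BP_PlayerCharacter and caches the reference.
; On overlap with that cached player, it adds its Ammo value directly to the TotalAmmo of the player's WeaponReference, then destroys itself.
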(event `self.ReceiveBeginPlay`
  (bind _asbp_player_character (cast `/Game/Core/Player/BP_PlayerCharacter` (`GameplayStatics.GetPlayerCharacter` 0)))
  (bind _output_get (set `self.PlayerReference` _asbp_player_character)))

(event `self.ReceiveActorBeginOverlap`
  (params (OtherActor :type "Actor Object Reference"))
  (if (== OtherActor (`self.PlayerReference`))
    (bind _weaponreference (`/Game/Core/Player/BP_PlayerCharacter.WeaponReference` (stale `self.ReceiveBeginPlay` _output_get)))
    (set `/Game/Weapons/Core/Blueprints/BP_WeaponSystem.TotalAmmo` (+ (`/Game/Weapons/Core/Blueprints/BP_WeaponSystem.TotalAmmo` _weaponreference) (`self.Ammo`)) _weaponreference)
    (`self.K2_DestroyActor`)))

(fn `UserConstructionScript`)