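; BP_StatTrack holds gameplay stat counters for bullets fired, reloads, kills and time played, and shows them for debugging or review.
; Tick runs through a one-second Delay to increment TimePlayed, giving an approximate seconds counter.
; Pressing Tab prints all four stats with PrintString.
; This graph only reads the bullet, reload and kill counters and never updates them.
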(event `self.ReceiveTick`
  (params (DeltaSeconds :type "Float (single-precision)"))
  (`KismetSystemLibrary.Delay` 1.0)
  (`/Engine/EditorBlueprintResources/StandardMacros.IncrementFloat` (`self.TimePlayed`)))

(event `Key|Tab`
  (params (Key :type "Key Structure"))
  (:`Pressed`
    (`KismetSystemLibrary.PrintString` (`KismetStringLibrary.Concat_StrStr` "Bullets Fired: " (`KismetStringLibrary.Conv_IntToString` (`self.BulletsFired`))))
    (`KismetSystemLibrary.PrintString` (`KismetStringLibrary.Concat_StrStr` "Total Reloads: " (`KismetStringLibrary.Conv_IntToString` (`self.TotalReloads`))))
    (`KismetSystemLibrary.PrintString` (`KismetStringLibrary.Concat_StrStr` "Time Played: " (`KismetStringLibrary.Conv_DoubleToString` (`self.TimePlayed`))))
    (`KismetSystemLibrary.PrintString` (`KismetStringLibrary.Concat_StrStr` "Kills: " (`KismetStringLibrary.Conv_IntToString` (`self.KillCounter`))))))

(fn `UserConstructionScript`)